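; BP_enemyParent is an enemy base that chases the player once seen, attacks, and dies from damage.
; PawnSensing starts a repeating AIMoveTo chase, and death notifies BP_EnemySpawner, increments player Kills and destroys the actor.
; An OnAttack binding, noted as not working, plays a random montage, then briefly disables movement.
; The montage notify runs a debug-drawn sphere overlap, damaging the player once per overlapped pawn, whoever it is.
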(event `self.PawnSensing.OnSeePawn`
  (params (Pawn :type "Pawn Object Reference"))
  (set `self.isSeeingPlayer` true)
  (`self.Roaming`))

(event `Roaming`
  (if (`self.isSeeingPlayer`)
    (`|AIMoveTo` self (0.0 0.0 0.0) (`GameplayStatics.GetPlayerCharacter` 0)
      (:`OnSuccess`
        (`KismetSystemLibrary.Delay` 0.2)
        (`self.Roaming`)))))

(event `self.ReceiveAnyDamage`
  (params (Damage :type "Float (single-precision)") (DamageType :type "DamageType Object Reference") (InstigatedBy :type "Controller Object Reference") (DamageCauser :type "Actor Object Reference"))
  (bind _output_get (set `self.Health` (- (`self.Health`) Damage)))
  (if (<= _output_get 0.0)
    (bind _returnvalue (`GameplayStatics.GetActorOfClass` "/Game/blueprints/spawners/BP_EnemySpawner.BP_EnemySpawner_C"))
    (bind _asbp_enemy_spawner (cast `/Game/blueprints/spawners/BP_EnemySpawner` _returnvalue))
    (`/Game/blueprints/spawners/BP_EnemySpawner.EnemyCounter` _asbp_enemy_spawner)
    (`|ExecutionSequence`
      (:`then_0`
        (bind _asbp_first_person_character (cast `/Game/FirstPerson/Blueprints/BP_FirstPersonCharacter` (`GameplayStatics.GetPlayerCharacter` 0)))
        (`/Engine/EditorBlueprintResources/StandardMacros.IncrementInt` (`/Game/FirstPerson/Blueprints/BP_FirstPersonCharacter.kills` _asbp_first_person_character)))
      (:`then_1`
        (`self.K2_DestroyActor`)))))

(event `self.ReceiveBeginPlay`
  (add `self.OnAttack` (delegate `attack`)))

(event `attack`
  (bind _attackanim (`self.attackanim`))
  ;[1 1 1] niedzialajacy atak
  (`/Engine/EditorBlueprintResources/StandardMacros.DoOnce` false :!label _label
    (:`Completed`
      (`|PlayMontage` (`self.Mesh`) (`|GetArrayItem` _attackanim (`KismetMathLibrary.RandomInteger` (`KismetArrayLibrary.Array_Length` _attackanim)))
        (:`OnCompleted`
          (`CharacterMovementComponent.DisableMovement` (`self.CharacterMovement`))
          (`KismetSystemLibrary.Delay` 2.0)
          (`CharacterMovementComponent.SetMovementMode` (`self.CharacterMovement`) "MOVE_Walking" 0)
          (goto _label :!via `Reset`))
        (:`OnNotifyBegin`
          (`self.Damage`))))))

(event `Damage`
  (bind _returnvalue (`SceneComponent.K2_GetComponentLocation` (`self.AtackSphere`)))
  ;[1 1 1] deal damage
  (bind _outactors (`KismetSystemLibrary.SphereOverlapActors` _returnvalue (`self.AttacikRange`) (`|MakeArray` "ObjectTypeQuery3" :!type "EObjectTypeQuery Enum") "/Script/Engine.Actor" (`|MakeArray` self :!type "Actor Object Reference")))
  (`KismetSystemLibrary.DrawDebugSphere` _returnvalue (`self.AttacikRange`) 12 (struct :`R` 1.0 :`B` 0.020533 :`A` 1.0) 2.0)
  (for _ _outactors
    (if true
      (bind _asbp_first_person_character (cast `/Game/FirstPerson/Blueprints/BP_FirstPersonCharacter` (`GameplayStatics.GetPlayerCharacter` 0)))
      (`GameplayStatics.ApplyDamage` _asbp_first_person_character (`self.Base Damage`) (`self.GetController`) self "/Script/Engine.DamageType")
      (else
        (`GameplayStatics.ApplyDamage` null)))))

(fn `UserConstructionScript`)