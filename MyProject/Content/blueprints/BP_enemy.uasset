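; Enemy NPC that chases the player after spotting them and carries a health bar widget.
; Pawn sensing sets a sight flag, never cleared here, and starts Roaming, which re-issues AI MoveTo toward the player after each successful move and short delay.
; BeginPlay copies Health into the widget.
; Overlaps with other BP_enemy actors toggle bar visibility: HealthBar begin shows it, Healthradious end hides it.
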(event `self.ReceiveBeginPlay`
  (bind _aswb_npc_health (cast `/Game/blueprints/WB_NPC_Health` (`WidgetComponent.GetUserWidgetObject` (`self.HealthBar`))))
  (bind _output_get (set `self.HealthbarRef` _aswb_npc_health))
  (set `/Game/blueprints/WB_NPC_Health.Health` (`self.Health`) _output_get))

(event `self.PawnSensing.OnSeePawn`
  (params (Pawn :type "Pawn Object Reference"))
  (set `self.isSeeingPlayer` true)
  (`self.Roaming`))

(event `Roaming`
  (if (`self.isSeeingPlayer`)
    (`|AIMoveTo` self (0.0 0.0 0.0) (`GameplayStatics.GetPlayerCharacter` 0)
      (:`OnSuccess`
        (`KismetSystemLibrary.Delay` 0.2)
        (`self.Roaming`)))))

(event `self.HealthBar.OnComponentBeginOverlap`
  (params (OverlappedComponent :type "PrimitiveComponent Object Reference") (OtherActor :type "Actor Object Reference") (OtherComp :type "PrimitiveComponent Object Reference") (OtherBodyIndex :type Integer) (bFromSweep :type Boolean) (SweepResult :type "HitResult Structure (by ref)"))
  (cast `/Game/blueprints/BP_enemy` OtherActor)
  (`SceneComponent.SetVisibility` (`self.HealthBar`) true false))

(event `self.healthradious.OnComponentEndOverlap`
  (params (OverlappedComponent :type "PrimitiveComponent Object Reference") (OtherActor :type "Actor Object Reference") (OtherComp :type "PrimitiveComponent Object Reference") (OtherBodyIndex :type Integer))
  (cast `/Game/blueprints/BP_enemy` OtherActor)
  (`SceneComponent.SetVisibility` (`self.HealthBar`) false false))

(fn `UserConstructionScript`)