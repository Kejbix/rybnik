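; Wave spawner actor that spawns AI enemies at random reachable navmesh points around itself, starting shortly after BeginPlay.
; An enemy-counter dispatcher decrements the remaining count; at zero it triggers the player's wave-start widget and grows the spawn count by half.
; It then fires its spawn dispatcher, which spawns the next wave after a delay.
; A separate endless delay loop periodically drops an Apteczka (first-aid kit) pickup nearby.
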(event `self.ReceiveBeginPlay`
  (`KismetSystemLibrary.Delay` 3.0)
  (`|ExecutionSequence`
    (:`then_0`
      (for _ (range 1 (+ (`self.spawn count`) 1))
        (`AIBlueprintHelperLibrary.SpawnAIFromClass` "/Game/blueprints/enemy/BP_enemyParent.BP_enemyParent_C" null (`NavigationSystemV1.K2_GetRandomReachablePointInRadius` (`self.K2_GetActorLocation`) 7000.0 null null) (struct) false null))
      (set `self.Enemies` (`self.spawn count`)))
    (:`then_1`
      (add `self.EnemyCounter` (delegate `DecrementEnemies`)))
    (:`then_2`
      (add `self.spawnenemies` (delegate `spawningWave`)))
    (:`then_3`
      (`KismetSystemLibrary.Delay` 20.0 :!label _label)
      (`|SpawnActorFromClass` "/Game/Apteczka.Apteczka_C" (`KismetMathLibrary.Conv_VectorToTransform` (`NavigationSystemV1.K2_GetRandomReachablePointInRadius` (`self.K2_GetActorLocation`) 3000.0 null null)) "AdjustIfPossibleButAlwaysSpawn" "MultiplyWithRoot" null null)
      (goto _label))))

(event `DecrementEnemies`
  (`/Engine/EditorBlueprintResources/StandardMacros.DecrementInt` (`self.Enemies`)
    (:`  `
      (if (<= (`self.Enemies`) 0)
        (bind _asbp_first_person_character (cast `/Game/FirstPerson/Blueprints/BP_FirstPersonCharacter` (`GameplayStatics.GetPlayerPawn` 0)))
        (`/Game/FirstPerson/Blueprints/BP_FirstPersonCharacter.startWaveWidget` _asbp_first_person_character)
        (bind _output_get (set `self.spawn count` (`KismetMathLibrary.Conv_Int64ToInt` (`KismetMathLibrary.Conv_DoubleToInt64` (* (`self.spawn count`) 1.5)))))
        (set `self.Enemies` _output_get)
        (`self.spawnenemies`)))))

(event `spawningWave`
  (`KismetSystemLibrary.Delay` (`self.delay between waves`))
  (for _ (range 1 (+ (`self.spawn count`) 1))
    (`AIBlueprintHelperLibrary.SpawnAIFromClass` "/Game/blueprints/enemy/BP_enemyParent.BP_enemyParent_C" null (`NavigationSystemV1.K2_GetRandomReachablePointInRadius` (`self.K2_GetActorLocation`) 7000.0 null null) (struct) false null)))

(fn `UserConstructionScript`)